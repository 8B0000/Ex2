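; UMP45 submachine gun weapon Blueprint with a gun mesh and sight and barrel attachment points.
; On BeginPlay, the IsBuyable flag enables query and physics collision on the mesh, or disables it otherwise.
; Every Tick, it snaps the mesh and both attachment points to one of two hardcoded relative positions, sitting lower when HasSight is true.
; Its GetInteractType function always returns "None".
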(event EventBeginPlay
  (if (Variables|Default|GetIsBuyable)
    (Collision|SetCollisionEnabled (Variables|Default|Getump45) "QueryAndPhysics")
    (else
      (Collision|SetCollisionEnabled (Variables|Default|Getump45) "NoCollision"))))

(event Collision|EventActorBeginOverlap
  (params (OtherActor :type Actor%20Object%20Reference)))

(event EventTick
  (params (DeltaSeconds :type Float%20%28single-precision%29))
  (if (Variables|Default|GetHasSight)
    (Transformation|SetRelativeLocation (Variables|Default|Getump45) "46.512608,0.000283,-23.902264" false false)
    (Transformation|SetRelativeLocation (Variables|Default|GetSightAttachmentPoint) "56.512608,0.000283,-2.902266" false false)
    (Transformation|SetRelativeLocation (Variables|Default|GetBarrelAttachmentPoint) "56.512608,0.000283,-1.902267" false false)
    (else
      (Transformation|SetRelativeLocation (Variables|Default|Getump45) "46.512608,0.000283,-18.380852" false false)
      (Transformation|SetRelativeLocation (Variables|Default|GetSightAttachmentPoint) "56.512608,0.000283,2.619146" false false)
      (Transformation|SetRelativeLocation (Variables|Default|GetBarrelAttachmentPoint) "56.512608,0.000283,3.619145" false false))))

(fn ConstructionScript)

(fn GetInteractType
  (params (Actor :type Actor%20Object%20Reference))
  (return "None"))