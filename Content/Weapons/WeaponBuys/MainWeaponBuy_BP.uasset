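; Base logic for a purchasable weapon pickup that sells its referenced weapon to the player for points.
; Overlap registers or clears it as the player's interaction target while buyable.
; Interaction checks points, swaps the weapon into the selected slot unless either slot already holds it, then deducts the price.
; Limited buys decrement their remaining count before those checks, so failed attempts also consume stock.
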(event EventInteraction
  (bind _weaponreference (Variables|Default|GetWeaponReference))
  ;[1 1 1] Interacting Code
  (if (and (Collision|IsOverlappingActor (Variables|Default|GetCollision) (Game|Player|GetPlayerPawn 0) :!class /Script/Engine.PrimitiveComponent) (Variables|Default|GetIsBuyable))
    (bind _asfirst_person_character (Utilities|Casting|CastToFirstPersonCharacter (Game|Player|GetPlayerPawn 0)))
    (if (Variables|Default|GetIsLimited)
      (if (> (Variables|Default|GetPurchaseLimit) 0)
        (Variables|Default|SetPurchaseLimit (- (Variables|Default|GetPurchaseLimit) 1))
        (if (>= (Variables|/Game/FirstPersonBP/Blueprints/FirstPersonCharacter.FirstPersonCharacter_C|GetPoints _asfirst_person_character) (Variables|Default|GetPrice)) :!label _label
          (if (Math|Boolean|ANDBoolean (!= (Variables|/Game/FirstPersonBP/Blueprints/FirstPersonCharacter.FirstPersonCharacter_C|GetWeaponSlot1 _asfirst_person_character) (Variables|Default|GetWeaponReference)) (== (Variables|/Game/FirstPersonBP/Blueprints/FirstPersonCharacter.FirstPersonCharacter_C|GetSelectedSlot _asfirst_person_character) 1) (!= (Variables|/Game/FirstPersonBP/Blueprints/FirstPersonCharacter.FirstPersonCharacter_C|GetWeaponSlot2 _asfirst_person_character) (Variables|Default|GetWeaponReference)))
            (Variables|/Game/FirstPersonBP/Blueprints/FirstPersonCharacter.FirstPersonCharacter_C|SetWeaponSlot1 _asfirst_person_character _weaponreference)
            (Default|UpdateSelectedWeapon _asfirst_person_character)
            (Variables|/Game/FirstPersonBP/Blueprints/FirstPersonCharacter.FirstPersonCharacter_C|SetPoints _asfirst_person_character (- (Variables|/Game/FirstPersonBP/Blueprints/FirstPersonCharacter.FirstPersonCharacter_C|GetPoints _asfirst_person_character) (Variables|Default|GetPrice)) :!label _label_2)
            (elif (Math|Boolean|ANDBoolean (== (Variables|/Game/FirstPersonBP/Blueprints/FirstPersonCharacter.FirstPersonCharacter_C|GetSelectedSlot _asfirst_person_character) 2) (!= (Variables|/Game/FirstPersonBP/Blueprints/FirstPersonCharacter.FirstPersonCharacter_C|GetWeaponSlot2 _asfirst_person_character) (Variables|Default|GetWeaponReference)) (!= (Variables|/Game/FirstPersonBP/Blueprints/FirstPersonCharacter.FirstPersonCharacter_C|GetWeaponSlot1 _asfirst_person_character) (Variables|Default|GetWeaponReference)))
              (Variables|/Game/FirstPersonBP/Blueprints/FirstPersonCharacter.FirstPersonCharacter_C|SetWeaponSlot2 _asfirst_person_character _weaponreference)
              (Default|UpdateSelectedWeapon _asfirst_person_character)
              (goto _label_2)
              (else
                (Development|PrintString "Both Failed Lol"))))
          (else
            (Development|PrintString "Not Enough Money"))))
      (else
        (goto _label)))))

(event Collision|EventActorBeginOverlap
  (params (OtherActor :type Actor%20Object%20Reference))
  ;[1 1 1] Interacting Code
  (if (and (== OtherActor (Game|GetPlayerCharacter 0)) (Variables|Default|GetIsBuyable))
    (bind _asfirst_person_character (Utilities|Casting|CastToFirstPersonCharacter (Game|Player|GetPlayerPawn 0)))
    (Default|Interactingwith _asfirst_person_character self)))

(event Collision|EventActorEndOverlap
  (params (OtherActor :type Actor%20Object%20Reference))
  ;[1 1 1] Interacting Code
  (if (== OtherActor (Game|GetPlayerCharacter 0))
    (bind _asfirst_person_character (Utilities|Casting|CastToFirstPersonCharacter (Game|Player|GetPlayerPawn 0)))
    (Default|InteractingEnd _asfirst_person_character)))

(fn ConstructionScript)