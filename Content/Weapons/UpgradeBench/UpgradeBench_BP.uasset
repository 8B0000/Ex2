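; UpgradeBench_BP is an interactable weapon upgrade bench that opens the player's upgrade bench through the first-person character.
; Overlap begin and end register and clear the bench as the character's current interaction target.
; Its Interaction event checks that the player pawn still overlaps the collision component, then calls UpgradeBenchOpen on FirstPersonCharacter, which handles the actual upgrade logic.
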(event EventInteraction
  (if (Collision|IsOverlappingActor (Variables|Default|GetCollisionComponent) (Game|Player|GetPlayerPawn 0) :!class /Script/Engine.PrimitiveComponent)
    (bind _asfirst_person_character (Utilities|Casting|CastToFirstPersonCharacter (Game|Player|GetPlayerPawn 0)))
    (Default|UpgradeBenchOpen _asfirst_person_character)))

(event Collision|EventActorBeginOverlap
  (params (OtherActor :type Actor%20Object%20Reference))
  (if (== OtherActor (Game|GetPlayerCharacter 0))
    (bind _asfirst_person_character (Utilities|Casting|CastToFirstPersonCharacter (Game|Player|GetPlayerPawn 0)))
    (Default|Interactingwith _asfirst_person_character self)))

(event Collision|EventActorEndOverlap
  (params (OtherActor :type Actor%20Object%20Reference))
  (if (== OtherActor (Game|GetPlayerCharacter 0))
    (bind _asfirst_person_character (Utilities|Casting|CastToFirstPersonCharacter (Game|Player|GetPlayerPawn 0)))
    (Default|InteractingEnd _asfirst_person_character)))

(fn ConstructionScript)