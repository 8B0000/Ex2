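; Base-style weapon Blueprint handling hitscan firing, magazine ammo, reloading and aim-down-sights.
; StartFire runs a looping timer into Fire, plus an immediate shot when Automatic; Fire gates on a delay, spends ammo, plays audio and line traces from Raycastspawn.
; The trace result is unused, so shots apply no damage.
; Reload refills from reserve after a delay without clamping it at zero; aiming snaps the model between two offsets.
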(event Custom|Fire
  (bind _raycastspawn (Variables|Default|Getraycastspawn))
  (bind _returnvalue (Transformation|GetWorldLocation _raycastspawn))
  ;[1 1 1] Firing
  (if (> (Variables|Default|GetCurrentAmmo) 0)
    (if (Variables|Default|GetCanFire)
      (Variables|Default|SetCanFire false)
      (Utilities|FlowControl|Delay (Variables|Default|GetWeaponFireCap))
      (Variables|Default|SetCanFire true)
      (Variables|Default|SetCurrentAmmo (- (Variables|Default|GetCurrentAmmo) 1))
      (Audio|Components|Audio|Play (Variables|Default|Getweapongunshot) 0.0)
      (bind _outhit (Collision|LineTraceByChannel _returnvalue (+ _returnvalue (* (Math|Vector|GetForwardVector _raycastspawn) (Variables|Default|GetRange))) "TraceTypeQuery1" false (Utilities|Array|MakeArray (Variables|Default|GetParent)) "None"))
      (else
        (CallFunction|StopFire)))
    (else
      (Audio|Components|Audio|Play (Variables|Default|Getweapondry) 0.0)
      (Variables|Default|SetCanFire false)
      (CallFunction|StopFire))))

(event Custom|StopFire
  ;[1 1 1] Firing
  (Utilities|Time|ClearandInvalidateTimerbyHandle (stale Custom|StartFire _returnvalue)))

(event Custom|StartFire
  ;[1 1 1] Firing
  (if (Variables|Default|GetCanFire)
    (bind _returnvalue (Utilities|Time|SetTimerbyEvent (delegate Custom|Fire) (Variables|Default|GetAuto%20Fire%20Time) true))
    (if (Variables|Default|GetAutomatic)
      (CallFunction|Fire))))

(event Custom|AimStart
  ;[1 1 1] Aiming
  (Variables|Default|SetADS true)
  (Transformation|SetRelativeLocation (Variables|Default|Getweaponmodel) (Variables|Default|GetADSCoord) false false))

(event Custom|AimEnd
  ;[1 1 1] Aiming
  (Variables|Default|SetADS false)
  (Transformation|SetRelativeLocation (Variables|Default|Getweaponmodel) (Variables|Default|GetRegCoord) false false))

(event Custom|Reload
  (bind _magazinesize (Variables|Default|GetMagazineSize))
  ;[1 1 1] Reloading
  (if (Math|Boolean|ANDBoolean (Variables|Default|GetCanReload) (< (Variables|Default|GetCurrentAmmo) (Variables|Default|GetMagazineSize)) (> (Variables|Default|GetReserveSize) 0))
    (Variables|Default|SetCanFire false)
    (Variables|Default|SetCanReload false)
    (Utilities|FlowControl|Delay (Variables|Default|GetReloadTime))
    (Variables|Default|SetReserveSize (- (+ (Variables|Default|GetCurrentAmmo) (Variables|Default|GetReserveSize)) _magazinesize))
    (Variables|Default|SetCurrentAmmo _magazinesize)
    (Variables|Default|SetCanFire true)
    (Variables|Default|SetCanReload true)))

(event EventBeginPlay
  ;[1 1 1] BeginPlay
  (Audio|Components|Audio|Stop (Variables|Default|GetWeapongunshot))
  (Audio|Components|Audio|StopDelayed (Variables|Default|Getweapondry) 0.0)
  (Transformation|SetRelativeLocation (Variables|Default|Getweaponmodel) (Variables|Default|GetRegCoord) false false))

(fn ConstructionScript)